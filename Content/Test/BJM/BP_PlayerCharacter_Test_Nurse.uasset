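; Test Blueprint of a nurse player character, used to try out the summon slot UI and abilities.
; Its TestSummonSlot event shows the mouse cursor, enables touch events and grants the Aether Charge and Heal test abilities.
; It then loads a hard-coded four-card deck into the SummonComponent and refreshes the test summon panel through the LR player controller's player widget.
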(event `self.TestSummonSlot`
  (bind _returnvalue (`GameplayStatics.GetPlayerController` 0))
  (set `PlayerController.bShowMouseCursor` true _returnvalue)
  (set `PlayerController.bEnableTouchEvents` true _returnvalue)
  (`self.GrantTestAbility` "/Game/Test/BJM/GAS/GA_AetherCharge.GA_AetherCharge_C")
  (`self.GrantTestAbility` "/Game/Test/BJM/GAS/GA_Heal.GA_Heal_C")
  (`LRSummonComponent.LoadDeckData` (`self.SummonComponent`) (`|MakeArray` "Anubis" "CHAR_WARRIOR_02" "CHAR_ARCHER_03" "CHAR_WARRIOR_04" :!type "Name"))
  (bind _aslrplayer_controller (cast `LRPlayerController` (`GameplayStatics.GetPlayerController` 0)))
  (bind _returnvalue_2 (`LRPlayerController.GetPlayerWidget` _aslrplayer_controller))
  (`LRPlayerWidget.TestSummonPanelRefresh` _returnvalue_2))

(fn `UserConstructionScript`)