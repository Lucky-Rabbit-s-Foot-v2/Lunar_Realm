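; Backup test player character Blueprint that sets up a summon-slot test in the game.
; Its TestSummonSlot event grants attack, aether charge and heal test abilities, and turns on the mouse cursor and touch events.
; It then loads a hard-coded character deck into the SummonComponent and refreshes the summon panel on the LRPlayerWidget obtained from the LRControllerBase persistent widget.
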(event `self.TestSummonSlot`
  (bind _returnvalue (`GameplayStatics.GetPlayerController` 0))
  (`self.GrantTestAbility` "/Game/Test/BJM/GAS/GA_Attack.GA_Attack_C")
  (set `PlayerController.bShowMouseCursor` true _returnvalue)
  (set `PlayerController.bEnableTouchEvents` true _returnvalue)
  (`self.GrantTestAbility` "/Game/Test/BJM/GAS/GA_AetherCharge.GA_AetherCharge_C")
  (`self.GrantTestAbility` "/Game/Test/BJM/GAS/GA_Heal.GA_Heal_C")
  (`LRSummonComponent.LoadDeckData` (`self.SummonComponent`) (`|MakeArray` "CHAR_MAGE_01" "CHAR_WARRIOR_01" "CHAR_HERO_01" "CHAR_ARCHER_01" :!type "Name"))
  (bind _aslrcontroller_base (cast `LRControllerBase` (`GameplayStatics.GetPlayerController` 0)))
  (bind _returnvalue_2 (`LRControllerBase.GetPersistentWidget` _aslrcontroller_base))
  (bind _aslrplayer_widget (cast `LRPlayerWidget` _returnvalue_2))
  (`LRPlayerWidget.TestSummonPanelRefresh` _aslrplayer_widget))

(fn `UserConstructionScript`)