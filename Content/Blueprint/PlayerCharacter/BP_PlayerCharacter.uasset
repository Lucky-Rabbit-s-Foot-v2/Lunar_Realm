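; Player character Blueprint whose only active graph logic is a TestSummonSlot event used for testing.
; The event enables the mouse cursor and touch events on the first player controller, then grants the Aether Charge and Heal test abilities.
; An unwired chain, which never runs, would load a hardcoded deck into SummonComponent and refresh the test summon panel through the LRPlayerController's player widget.
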(event `self.TestSummonSlot`
  (bind _returnvalue (`GameplayStatics.GetPlayerController` 0))
  (set `PlayerController.bShowMouseCursor` true _returnvalue)
  (set `PlayerController.bEnableTouchEvents` true _returnvalue)
  (`self.GrantTestAbility` "/Game/Test/BJM/GAS/GA_AetherCharge.GA_AetherCharge_C")
  (`self.GrantTestAbility` "/Game/Test/BJM/GAS/GA_Heal.GA_Heal_C"))

(fn `UserConstructionScript`)